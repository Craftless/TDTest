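; Tower Blueprint that turns its turret toward the AI controller's enemy and fires homing projectiles on Attack.
; Tick smoothly interpolates turret rotation, skipping enemies very close to the muzzle.
; SpawnProjectile backs the spawn point away from close targets, sets damage from an attribute, runs projectile modifier objects and assigns the homing target.
; Modifiers register into separate projectile and self arrays; debug prints remain in the spawn path.
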(event EventBeginPlay
  (|CallParentFunction))

(event Collision|EventActorBeginOverlap
  (params (OtherActor :type Actor%20Object%20Reference))
  (|CallParentFunction OtherActor) ; This node is disabled and will not be called.\nDrag off pins to build functionality.
)

(event EventTick
  (params (DeltaSeconds :type Float%20%28single-precision%29))
  (|CallParentFunction DeltaSeconds)
  (CallFunction|MakeTurretLookatEnemy)
  (Variables|Default|SetAlpha (Math|Float|Clamp(Float) (+ (Variables|Default|GetAlpha) DeltaSeconds))))

(event EventAttack
  (params (TargetedActor :type Actor%20Object%20Reference))
  (|CallParentFunction TargetedActor)
  (CallFunction|SpawnProjectile TargetedActor (Variables|Default|GetProjectile%20Class)))

(fn ConstructionScript
  (|CallParentFunction))

(fn MakeTurretLookatEnemy
  (bind _aicontroller (Variables|Default|GetAIController)
    (:then
      (bind _enemy (Variables|/Game/AI/BP_TowerAIControllerBase.BP_TowerAIControllerBase_C|GetEnemy _aicontroller)
        (:then
          (if (not (<= (Class|KismetMathLibrary|VectorDistanceSquared (Transformation|GetActorLocation _enemy) (Transformation|GetWorldLocation (Variables|Default|GetProjectileSpawnPoint))) 2.5e+03))
            (CallFunction|TurretLookTowards (Math|Conversions|RotationFromXVector (Math|Vector|Normalize (- (Transformation|GetActorLocation _enemy) (Transformation|GetWorldLocation (Variables|Default|GetProjectileSpawnPoint))))))))
        (:else)))
    (:else)))

(fn SpawnProjectile
  (params (TargetedActor :type Actor%20Object%20Reference) (ProjectileClass :type BP%20Tower%20Generic%20Projectile%20Class%20Reference))
  (bind _returnvalue (Transformation|GetActorLocation TargetedActor))
  (bind (_asbp_enemy_base _bsuccess) (Utilities|Casting|CastToBP_EnemyBase TargetedActor))
  (bind _projectilespawnpoint (Variables|Default|GetProjectileSpawnPoint))
  (bind _projectilespawnpoint_2 (Variables|Default|GetProjectileSpawnPoint))
  (bind _returnvalue_2 (Transformation|GetWorldTransform _projectilespawnpoint))
  (bind _returnvalue_3 (Transformation|GetWorldLocation _projectilespawnpoint_2))
  (bind _returnvalue_4 (Class|KismetMathLibrary|VectorDistanceSquared _returnvalue _returnvalue_3))
  (bind _returnvalue_5 (<= _returnvalue_4 1e+04))
  (Development|PrintString (Utilities|String|ToString(Boolean) _returnvalue_5) true true "(R=1.000000,G=0.945428,B=0.000000,A=1.000000)")
  (bind _returnvalue_6 (Game|SpawnActorfromClass ProjectileClass (Math|Transform|MakeTransform (select _returnvalue_5 (+ _returnvalue_3 (* (Math|Vector|Normalize (- (Transformation|GetWorldLocation (Variables|Default|GetProjectileSpawnPoint)) (Transformation|GetActorLocation TargetedActor))) 5e+01)) _returnvalue_3) (.rotation _returnvalue_2) (.scale _returnvalue_2)) "AlwaysSpawn" self self))
  (Utilities|FlowControl|Sequence
    (:then_0
      (Utilities|IsValid _returnvalue_6
        (:Is%20Valid
          _)
        (:Is%20Not%20Valid
          (Development|PrintString (Utilities|String|Append "Proj Invalid" (Utilities|String|ToString(Float) (Utilities|Time|GetTimeSeconds))) true true "(R=1.000000,G=0.000000,B=0.072311,A=1.000000)")))
      (CallFunction|SetProjectileVariables _returnvalue_6)
      (Utilities|IsValid TargetedActor
        (:Is%20Valid
          (Default|SetHomingTarget _returnvalue_6 (select _bsuccess (Variables|/Script/TDTest.EnemyBase|GetTargetComp _asbp_enemy_base) (Actor|GetComponentbyClass TargetedActor "/Script/Engine.SceneComponent"))))))
    (:then_1
      (if _returnvalue_5
        (Variables|/Game/Blueprints/BP_Tower_GenericProjectile.BP_Tower_GenericProjectile_C|SetDRAW%20DEBUG _returnvalue_6 true)))))

(fn SetProjectileVariables
  (params (SpawnedProjectile :type BP%20Tower%20Generic%20Projectile%20Object%20Reference))
  (Utilities|FlowControl|Sequence
    (:then_0
      (Variables|/Game/Blueprints/BP_Tower_GenericProjectile.BP_Tower_GenericProjectile_C|SetDamageAmount SpawnedProjectile (Utilities|GetAttributeCurrentValue "(AttributeName=\"AttackDamage\",Attribute=/Script/TDTest.TowerAttributeSetBase:AttackDamage,AttributeOwner=None)")))
    (:then_1
      (Variables|Default|SetSpawnedProjectile SpawnedProjectile))
    (:then_2
      (for _array_element (Variables|Default|GetProjectileModifiers)
        (bind _returnvalue (Game|ConstructObjectfromClass _array_element self))
        (CallFunction|ExecuteModifier _returnvalue self 1)))))

(fn TurretLookTowards
  (params (Target :type Rotator))
  (bind _turret_t (Variables|Default|GetTurret_T))
  (Transformation|SetWorldRotation _turret_t (Math|Interpolation|RInterpTo (Transformation|GetWorldRotation _turret_t) Target (Utilities|Time|GetWorldDeltaSeconds) 5.0) false false))

(fn AddtoModifierArray
  (params (Modifier :type BP%20Modifier%20Class%20Reference) (ModifierArray :type EModifierArray%20Enum :default "NewEnumerator0"))
  (Utilities|Array|AddUnique (Utilities|Select :Index ModifierArray :NewEnumerator0 (Variables|Default|GetProjectileModifiers) :NewEnumerator1 (Variables|Default|GetSelfModifiers)) Modifier)
  (return))