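; Tower defense game mode that builds the tile map at BeginPlay, then spawns the first enemy wave.
; ConstructTiles parses the TileLayout string character by character into a grid of usable, path, start and end tiles.
; StartWaves parses WaveLayout's first entry, where letters spawn basic or fast enemies and digits add delays, retrying a limited number of times when spawning fails.
; Spawned enemies are tracked until killed; SpawnWaves is an uncalled alternative loop.
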(event Custom|SpawnWaves
  (bind _output_get (Variables|Default|SetArrayed (Utilities|String|GetCharacterArrayfromString (Utilities|String|ToString(Text) (Utilities|Array|Get(acopy) (Variables|Default|GetWaveLayout))))))
  (for _array_element _output_get
    (Utilities|FlowControl|Delay 5.0)
    (switch string (Utilities|Array|Get(acopy) (Variables|Default|GetArrayed))
      (:Default
        (if (> (Math|Conversions|ToInteger(Byte) (Utilities|Array|Get(acopy) (Variables|Default|GetArrayed))) 0)
          (Utilities|FlowControl|Delay (Math|Conversions|ToFloat(Integer) (Math|Conversions|ToInteger(Byte) (Utilities|Array|Get(acopy) (Variables|Default|GetArrayed)))))
          (else
            (Development|PrintString "FALSED"))))
      (:B
        (bind _success (CallFunction|SpawnEnemy "/Game/Blueprints/BP_EnemyBase_BasicEnemy.BP_EnemyBase_BasicEnemy_C" :!label _label))
        (if _success
          (Development|PrintString "Fourth")
          (Variables|Default|SetSpawnCounter 0)
          (Development|PrintString "Spawned" true true "(R=0.000000,G=0.092902,B=1.000000,A=1.000000)")
          (else
            (Development|PrintString "Fifth")
            (Math|Integer|IncrementInt (Variables|Default|GetSpawnCounter)
              (:%20%20
                (if (< (Variables|Default|GetSpawnCounter) 30)
                  (Utilities|FlowControl|Delay 0.2)
                  (goto _label)
                  (else
                    (Development|PrintString "Unable to spawn" true true "(R=1.000000,G=0.013981,B=0.000000,A=1.000000)" 1e+01))))))))))
  (Development|PrintString "Completed"))

(event Custom|StartWaves
  (bind _output_get (Variables|Default|SetArrayed (Utilities|String|GetCharacterArrayfromString (Utilities|String|ToString(Text) (Utilities|Array|Get(acopy) (Variables|Default|GetWaveLayout))))))
  (if (> (Utilities|Array|Length _output_get) 0) :!label _label
    (Utilities|FlowControl|Sequence
      (:then_0
        (switch string (Utilities|Array|Get(acopy) (Variables|Default|GetArrayed))
          (:Default
            (if (> (Math|Conversions|ToInteger(Byte) (Utilities|Array|Get(acopy) (Variables|Default|GetArrayed))) 0)
              (Utilities|FlowControl|Delay (Math|Conversions|ToFloat(Integer) (Math|Conversions|ToInteger(Byte) (Utilities|Array|Get(acopy) (Variables|Default|GetArrayed)))))
              (else
                (Development|PrintString "FALSED")))
            (Utilities|Array|RemoveIndex (Variables|Default|GetArrayed) :!label _label_2)
            (Utilities|FlowControl|Delay 0.2)
            (goto _label))
          (:B
            (bind (_spawningsuccess _spawned_enemy) (Utilities|TrySpawnEnemy "/Game/Blueprints/BP_EnemyBase_BasicEnemy.BP_EnemyBase_BasicEnemy_C" :!label _label_3)
              (:Clear
                (if _spawningsuccess
                  (Variables|Default|SetSpawnCounter 0)
                  (Utilities|Array|AddUnique (Variables|Default|GetEnemies) _spawned_enemy)
                  (goto _label_2)
                  (else
                    _)))
              (:NotClear
                _))
            (Math|Integer|IncrementInt (Variables|Default|GetSpawnCounter)
              (:%20%20
                (if (< (Variables|Default|GetSpawnCounter) 30)
                  (Utilities|FlowControl|Delay 0.2)
                  (goto _label_3)
                  (else
                    (Development|PrintString "Unable to spawn" true true "(R=1.000000,G=0.013981,B=0.000000,A=1.000000)" 1e+01))))))
          (:f
            (bind (_spawningsuccess_2 _spawned_enemy_2) (Utilities|TrySpawnEnemy "/Game/Blueprints/BP_EnemyBase_BasicEnemy_Fast.BP_EnemyBase_BasicEnemy_Fast_C" :!label _label_4)
              (:Clear
                (Utilities|UpdateSpawnEnemy _spawningsuccess_2 _spawned_enemy_2 :!label _label_5
                  (:TrueCompleted
                    (goto _label_2))
                  (:FalseCompleted
                    (goto _label_4))))
              (:NotClear
                (goto _label_5 StraightToFailed)))))))
    (else
      (Development|PrintString (Utilities|String|Append "Done" (Utilities|String|ToString(Integer) (Utilities|Array|Length (Variables|Default|GetArrayed)))) true true "(R=0.276985,G=1.000000,B=0.000000,A=1.000000)"))))

(event EventBeginPlay
  (Utilities|Time|SetGlobalTimeDilation 1.0)
  (CallFunction|ConstructTiles "0, 0, 0")
  (CallFunction|StartWaves))

(event EventTick
  (params (DeltaSeconds :type Float%20%28single-precision%29)))

(fn ConstructionScript)

(fn ConstructTiles
  (params (StartLocation :type Vector))
  (bind _output_get (LocalVariables|SetArrayed (Utilities|String|GetCharacterArrayfromString (Utilities|String|ToString(Text) (Variables|Default|GetTileLayout)))))
  (while (> (Utilities|Array|Length _output_get) 0)
    (Utilities|FlowControl|Sequence
      (:then_0
        (switch string (Utilities|Array|Get(acopy) (LocalVariables|GetArrayed))
          (:,
            (LocalVariables|SetSpawnOffset (- (LocalVariables|GetSpawnOffset) (Math|Vector|MakeVector 1e+02 (LocalVariables|GetRowOffset) 0.0)))
            (LocalVariables|SetRowOffset 0.0))
          (:U
            (LocalVariables|SetRowOffset (+ (LocalVariables|GetRowOffset) 1e+02))
            (LocalVariables|SetSpawnOffset (+ (LocalVariables|GetSpawnOffset) "0.000000,100.000000, 0"))
            (Game|SpawnActorfromClass "/Game/Blueprints/BP_UsableTile.BP_UsableTile_C" (Math|Transform|MakeTransform (+ StartLocation (LocalVariables|GetSpawnOffset)) "0, 0, 0" "1,1,1") "Undefined" 0 0))
          (:P
            (LocalVariables|SetRowOffset (+ (LocalVariables|GetRowOffset) 1e+02))
            (LocalVariables|SetSpawnOffset (+ (LocalVariables|GetSpawnOffset) "0.000000,100.000000, 0"))
            (Game|SpawnActorfromClass "/Game/Blueprints/BP_PathTIle.BP_PathTile_C" (Math|Transform|MakeTransform (+ StartLocation (LocalVariables|GetSpawnOffset)) "0, 0, 0" "1,1,1") "Undefined" 0 0))
          (:E
            (LocalVariables|SetRowOffset (+ (LocalVariables|GetRowOffset) 1e+02))
            (LocalVariables|SetSpawnOffset (+ (LocalVariables|GetSpawnOffset) "0.000000,100.000000, 0"))
            (Game|SpawnActorfromClass "/Game/Blueprints/BP_PathTIle_End.BP_PathTile_End_C" (Math|Transform|MakeTransform (+ StartLocation (LocalVariables|GetSpawnOffset)) "0, 0, 0" "1,1,1") "Undefined" 0 0))
          (:S
            (LocalVariables|SetRowOffset (+ (LocalVariables|GetRowOffset) 1e+02))
            (LocalVariables|SetSpawnOffset (+ (LocalVariables|GetSpawnOffset) "0.000000,100.000000, 0"))
            (bind _returnvalue (Game|SpawnActorfromClass "/Game/Blueprints/BP_PathTIle_Start.BP_PathTile_Start_C" (Math|Transform|MakeTransform (+ StartLocation (LocalVariables|GetSpawnOffset)) "0, 0, 0" "1,1,1") "Undefined" 0 0))
            (Variables|Default|SetStartTile _returnvalue))))
      (:then_1
        (Utilities|Array|RemoveIndex (LocalVariables|GetArrayed))))))

(fn SpawnEnemy
  (params (EnemyClass :type Enemy%20Base%20Class%20Reference))
  (bind _starttile (Variables|Default|GetStartTile))
  (bind _returnvalue (Transformation|GetActorTransform _starttile))
  (if (Variables|/Game/Blueprints/BP_PathTIle_Start.BP_PathTile_Start_C|GetIsClear (Variables|Default|GetStartTile))
    (bind _returnvalue_2 (Game|SpawnActorfromClass EnemyClass (Math|Transform|MakeTransform (- (.location _returnvalue) (.SpawningOffset (Utilities|GetClassDefaults EnemyClass))) (.rotation _returnvalue) (.scale _returnvalue)) "DontSpawnIfColliding" 0 0))
    (return (Utilities|IsValid _returnvalue_2) _returnvalue_2)))

(fn OnEnemyKilled
  (params (Enemy :type Enemy%20Base%20Object%20Reference))
  (bind _enemies (Variables|Default|GetEnemies))
  (Utilities|Array|RemoveItem _enemies Enemy)
  (if (<= (Utilities|Array|Length _enemies) 0)
    (Development|PrintString "Wave Cleared" true true "(R=1.000000,G=0.567433,B=0.071117,A=1.000000)")))