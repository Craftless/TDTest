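; BP_PathTIle_Start is a path start tile that shows whether enemies are currently occupying it.
; Box overlap events maintain a list of overlapping EnemyBase actors, and UpdateIsClear sets IsClear when that list is empty.
; BeginPlay applies a dynamic instance of M_TileMaterial to the mesh, and Tick sets its Colour parameter green when clear or red when occupied.
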(event OnComponentBeginOverlap(Box)
  (params (OverlappedComponent :type Primitive%20Component%20Object%20Reference) (OtherActor :type Actor%20Object%20Reference) (OtherComp :type Primitive%20Component%20Object%20Reference) (OtherBodyIndex :type Integer) (bFromSweep :type Boolean) (SweepResult :type Hit%20Result%20Structure%20%28by%20ref%29))
  (if (Utilities|ClassIsChildOf (Utilities|GetClass OtherActor) "/Script/TDTest.EnemyBase")
    (Utilities|Array|AddUnique (Variables|Default|GetOverlappedActors) OtherActor)
    (CallFunction|UpdateIsClear)))

(event OnComponentEndOverlap(Box)
  (params (OverlappedComponent :type Primitive%20Component%20Object%20Reference) (OtherActor :type Actor%20Object%20Reference) (OtherComp :type Primitive%20Component%20Object%20Reference) (OtherBodyIndex :type Integer))
  (Utilities|Array|RemoveItem (Variables|Default|GetOverlappedActors) OtherActor)
  (CallFunction|UpdateIsClear))

(event EventBeginPlay
  (|CallParentFunction)
  (CallFunction|UpdateIsClear)
  (bind _returnvalue (Rendering|Material|CreateDynamicMaterialInstance "/Game/Materials/M_TileMaterial.M_TileMaterial" "None" "None" :!class /Script/Engine.KismetMaterialLibrary))
  (bind _output_get (Variables|Default|SetDynMat _returnvalue))
  (Rendering|Material|SetMaterial (Variables|Default|GetStaticMesh) 0 _output_get))

(event Collision|EventActorBeginOverlap
  (params (OtherActor :type Actor%20Object%20Reference))
  (|CallParentFunction OtherActor) ; This node is disabled and will not be called.\nDrag off pins to build functionality.
)

(event EventTick
  (params (DeltaSeconds :type Float%20%28single-precision%29))
  (|CallParentFunction DeltaSeconds)
  (Rendering|Material|SetVectorParameterValue (Variables|Default|GetDynMat) "Colour" (select (Variables|Default|GetIsClear) "(R=0.000000,G=1.000000,B=0.019941,A=1.000000)" "(R=1.000000,G=0.000000,B=0.000000,A=1.000000)") :!class /Script/Engine.MaterialInstanceDynamic))

(fn ConstructionScript
  (|CallParentFunction))

(fn UpdateIsClear
  (Variables|Default|SetIsClear (<= (Utilities|Array|Length (Variables|Default|GetOverlappedActors)) 0)))