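; Tower defense build tile that highlights on mouse hover and handles input for the tower placed on it.
; A dynamic material swaps its Colour parameter on hover and restores the cached original afterward.
; While hovered, number keys pick a class from the GameMode's Towers list, spawned through a ChildActor component if empty and the player's gold spend succeeds.
; Left click toggles the tower's menu and right click sells it.
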(event EventBeginPlay
  (|CallParentFunction)
  (bind _output_get (Variables|Default|SetTemp (Utilities|Array|Get(acopy) (Rendering|Material|GetMaterials (Variables|Default|GetStaticMesh)))))
  (bind _returnvalue (Rendering|Material|CreateDynamicMaterialInstance _output_get "None" "None" :!class /Script/Engine.KismetMaterialLibrary))
  (bind _output_get_2 (Variables|Default|SetDynMat _returnvalue))
  (Rendering|Material|SetMaterial (Variables|Default|GetStaticMesh) 0 _output_get_2)
  (bind _returnvalue_2 (Rendering|Material|GetVectorParameterValue (Variables|Default|GetDynMat) "Colour" :!class /Script/Engine.MaterialInstanceDynamic))
  (Variables|Default|SetOriginalColour _returnvalue_2))

(event Collision|EventActorBeginOverlap
  (params (OtherActor :type Actor%20Object%20Reference)))

(event EventTick
  (params (DeltaSeconds :type Float%20%28single-precision%29)))

(event EventOnKeyPressedWhileHovering
  (params (KeyPressed :type Key%20Structure%20%28by%20ref%29) (Player :type Player%20Pawn%20Object%20Reference))
  (|CallParentFunction KeyPressed Player)
  (if (== KeyPressed "RightMouseButton")
    (CallFunction|SellTower)
    (elif (== KeyPressed "LeftMouseButton")
      (bind _spawnedtower (Variables|Default|GetSpawnedTower)
        (:then
          (bind _widgetblueprint (Variables|/Game/Blueprints/BP_Tower.BP_Tower_C|GetWidgetBlueprint _spawnedtower)
            (:then
              (Default|ShowMenu _spawnedtower (not (Widget|IsVisible _widgetblueprint))))
            (:else
              (Default|ShowMenu _spawnedtower true))))
        (:else))
      (else
        (CallFunction|ConvertKeytoNumber KeyPressed Player)))))

(event EventOnMouseStartHovered
  (|CallParentFunction)
  (Rendering|Material|SetVectorParameterValue (Variables|Default|GetDynMat) "Colour" "(R=1.000000,G=0.705901,B=0.297205,A=1.000000)" :!class /Script/Engine.MaterialInstanceDynamic))

(event EventOnMouseStopHovered
  (|CallParentFunction)
  (Rendering|Material|SetVectorParameterValue (Variables|Default|GetDynMat) "Colour" (Variables|Default|GetOriginalColour) :!class /Script/Engine.MaterialInstanceDynamic))

(fn ConstructionScript)

(fn SpawnTower
  (params (InClass :type BP%20Tower%20Class%20Reference) (User :type Player%20Pawn%20Object%20Reference))
  (bind _childactor (Variables|Default|GetChildActor))
  (Variables|/Script/Engine.ChildActorComponent|GetChildActor _childactor
    (:then)
    (:else
      (bind _returnvalue (Class|PlayerPawn|SpendGold User (.GoldCost (Utilities|GetClassDefaults InClass))))
      (if _returnvalue
        (ChildActorComponent|SetChildActorClass _childactor InClass)
        (bind _asbp_tower (Utilities|Casting|CastToBP_Tower (Variables|/Script/Engine.ChildActorComponent|GetChildActor (Variables|Default|GetChildActor))))
        (bind _output_get (Variables|Default|SetSpawnedTower _asbp_tower))
        (Variables|/Script/TDTest.Tower|SetOwnerPlayer _output_get User)
        (Actor|SetOwner _output_get User)))))

(fn SellTower
  (bind _spawnedtower (Variables|Default|GetSpawnedTower)
    (:then
      (Class|Tower|Sell _spawnedtower))
    (:else)))

(fn ConvertKeytoNumber
  (params (Key :type Key%20Structure%20%28by%20ref%29) (User :type Player%20Pawn%20Object%20Reference))
  (bind _returnvalue (Class|KismetInputLibrary|KeyGetDisplayName Key))
  (bind _gamemode (Variables|Default|GetGameMode))
  (bind _returnvalue_2 (Utilities|String|ToString(Text) _returnvalue))
  (bind _towers (Variables|/Game/Blueprints/BP_TDClassicGameMode.BP_TDClassicGameMode_C|GetTowers _gamemode))
  (bind _returnvalue_3 (Math|Conversions|ToInteger(Byte) _returnvalue_2))
  (if (not (<= _returnvalue_3 0))
    (if (>= (Utilities|Array|Length _towers) _returnvalue_3)
      (CallFunction|SpawnTower (Utilities|Array|Get(acopy) _towers (- _returnvalue_3 1)) User))))