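; BP_Tower_Archer is an archer tower Blueprint that receives elemental projectile upgrade paths when play begins.
; After calling its parent BeginPlay and waiting briefly, it adds two paths to itself, one granting a burning projectile modifier and one a cold projectile modifier.
; Unconnected leftover nodes would add path points or apply a Burn ability modifier directly, but never run.
; The construction script only calls its parent.
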(event EventBeginPlay
  (|CallParentFunction)
  (Utilities|FlowControl|Delay 0.2)
  (bind _constructed_path (CallFunction|AddPathtoActor self "/Game/Blueprints/Paths/BP_Path_GrantModifier_BurningProjectile.BP_Path_GrantModifier_BurningProjectile_C"))
  (CallFunction|AddPathtoActor self "/Game/Blueprints/Paths/BP_Path_GrantModifier_ColdProjectile.BP_Path_GrantModifier_ColdProjectile_C"))

(event Collision|EventActorBeginOverlap
  (params (OtherActor :type Actor%20Object%20Reference))
  (|CallParentFunction OtherActor) ; This node is disabled and will not be called.\nDrag off pins to build functionality.
)

(fn ConstructionScript
  (|CallParentFunction))