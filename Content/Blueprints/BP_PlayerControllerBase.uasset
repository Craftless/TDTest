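; Player controller base that handles the gold HUD, camera zoom, tile key input and game speed.
; On possessing a BP_PlayerPawn, it caches the pawn and creates a WBP_Gold widget initialized with it.
; Zoom moves the pawn's camera along world Z, dividing out time dilation to keep scroll speed constant.
; Key presses are forwarded to the hovered tile, while Period raises global time dilation in steps.
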(event EventBeginPlay)

(event EventTick
  (params (DeltaSeconds :type Float%20%28single-precision%29)))

(event EventPossess
  (params (PossessedPawn :type Pawn%20Object%20Reference))
  (bind _asbp_player_pawn (Utilities|Casting|CastToBP_PlayerPawn PossessedPawn))
  (Variables|Default|SetPlayerPawn _asbp_player_pawn)
  (Utilities|FlowControl|Sequence
    (:then_0
      (bind _returnvalue (UserInterface|CreateWidget "/Game/UI/WBP_Gold.WBP_Gold_C" self))
      (UserInterface|Viewport|AddtoViewport _returnvalue 0)
      (Default|Initialise _returnvalue (Variables|Default|GetPlayerPawn)))))

(event Input|AxisEvents|InputAxisZoomIn
  (params (AxisValue :type Float%20%28single-precision%29))
  (bind _playerpawn (Variables|Default|GetPlayerPawn)
    (:then
      (Transformation|AddWorldOffset (Variables|/Game/Blueprints/BP_PlayerPawn.BP_PlayerPawn_C|GetCamera _playerpawn) (Math|Vector|MakeVector 0.0 0.0 (* (* (Variables|Default|GetCameraScrollSpeed) AxisValue) (/ (Utilities|Time|GetWorldDeltaSeconds) (Class|GameplayStatics|GetGlobalTimeDilation)))) false false))
    (:else)))

(event Input|KeyboardEvents|AnyKey
  (params (Key :type Key%20Structure :default "None"))
  (bind _playerpawn (Variables|Default|GetPlayerPawn))
  (:Pressed
    (bind _returnvalue (Class|PlayerPawn|GetHoveredTile _playerpawn))
    (Utilities|IsValid _returnvalue
      (:Is%20Valid
        (Class|Tile|OnKeyPressedWhileHovering _returnvalue Key _playerpawn)))))

(event Input|KeyboardEvents|Period
  (params (Key :type Key%20Structure :default "None"))
  (:Pressed
    (Utilities|Time|SetGlobalTimeDilation (+ (Class|GameplayStatics|GetGlobalTimeDilation) 0.5))))

(event Input|KeyboardEvents|Comma
  (params (Key :type Key%20Structure :default "None")))

(fn ConstructionScript)