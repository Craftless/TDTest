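; Generic tower projectile that can home on a target component and damages the actor it overlaps.
; Each tick it re-aims its movement velocity at any valid homing target, preserving speed.
; Overlapping a non-owner actor destroys it after applying damage through GAS: the instigator's ability system sends a health-grant effect with negative magnitude.
; Conditional modifier effects are attached to that damage spec first, with a debug print of each instigator.
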(event OnComponentBeginOverlap(Sphere1)
  (params (OverlappedComponent :type Primitive%20Component%20Object%20Reference) (OtherActor :type Actor%20Object%20Reference) (OtherComp :type Primitive%20Component%20Object%20Reference) (OtherBodyIndex :type Integer) (bFromSweep :type Boolean) (SweepResult :type Hit%20Result%20Structure%20%28by%20ref%29))
  (CallFunction|OnHit OtherActor))

(event EventBeginPlay)

(event Collision|EventActorBeginOverlap
  (params (OtherActor :type Actor%20Object%20Reference)))

(event EventTick
  (params (DeltaSeconds :type Float%20%28single-precision%29))
  (Utilities|FlowControl|Sequence
    (:then_0
      (bind _homingtarget (Variables|Default|GetHomingTarget)
        (:then
          (CallFunction|HomingBehaviour _homingtarget))
        (:else)))))

(fn ConstructionScript)

(fn SetHomingTarget
  (params (HomingComponent :type Scene%20Component%20Object%20Reference))
  (Variables|Default|SetHomingTarget HomingComponent))

(fn HomingBehaviour
  (params (HomingTarget :type Scene%20Component%20Object%20Reference))
  (bind _returnvalue (Transformation|GetWorldLocation HomingTarget))
  (bind _returnvalue_2 (Transformation|GetActorLocation))
  (bind _returnvalue_3 (Math|Rotator|FindLookatRotation _returnvalue_2 _returnvalue))
  (bind (_roll _pitch _yaw) (Math|Rotator|BreakRotator _returnvalue_3))
  (Variables|/Script/Engine.MovementComponent|SetVelocity (Variables|Default|GetProjectileMovement) (Class|KismetMathLibrary|CreateVectorfromYawPitch _yaw _pitch (Math|Vector|VectorLength (Transformation|GetVelocity)))))

(fn DamageActor
  (params (HitActor :type Actor%20Object%20Reference) (GEClass :type Gameplay%20Effect%20Class%20Reference))
  (bind _returnvalue (Game|GetInstigator))
  (bind _returnvalue_2 (Ability|GetAbilitySystemComponent _returnvalue))
  (Utilities|FlowControl|Sequence
    (:then_0
      (bind _gespec (CallFunction|CreateGameplayEffectSpecwithCallerMagnitude _returnvalue_2 "/Game/GameplayAbilities/Attributes/GE_GrantHealth.GE_GrantHealth_C" "(TagName=\"attributes.health.grant\")" (* -1 (Variables|Default|GetDamageAmount)))))
    (:then_1
      (for _array_element (Variables|Default|GetDamageActorConditionalModifiers)
        (bind _returnvalue_3 (Class|AbilitySystemBlueprintLibrary|GetEffectContext _array_element))
        (Development|PrintString (Utilities|GetDisplayName (Class|AbilitySystemBlueprintLibrary|EffectContextGetInstigatorActor _returnvalue_3)))
        (Class|GASFunctionLibrary|AddConditionalEffecttoSpec _gespec _array_element))
      (GameplayEffects|ApplyGameplayEffectSpecToTarget _returnvalue_2 _gespec (Ability|GetAbilitySystemComponent HitActor)))))

(fn OnHit
  (params (HitActor :type Actor%20Object%20Reference))
  (if (not (== HitActor (Components|GetOwner)))
    (CallFunction|DamageActor HitActor "/Game/GameplayAbilities/Attributes/GE_GrantHealth.GE_GrantHealth_C")
    (Actor|DestroyActor)))