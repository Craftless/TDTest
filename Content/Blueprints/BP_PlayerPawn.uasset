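; BP_PlayerPawn is the player's camera pawn for the tower defense game, holding Gold and a set of debug hotkeys.
; BeginPlay caches the classic game mode, sets starting Gold and starts a looping one-second timer, while RegenGold adds one gold per call.
; Movement axes pan the pawn, dividing out global time dilation to keep speed constant.
; Hotkeys change time dilation, rebuild navmeshes, fire an archer projectile, grant towers experience through GAS and test an array.
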(event EventBeginPlay
  (bind _asbp_tdclassic_game_mode (Utilities|Casting|CastToBP_TDClassicGameMode (Game|GetGameMode)))
  (Variables|Default|SetGameMode _asbp_tdclassic_game_mode)
  (Utilities|FlowControl|Sequence
    (:then_0
      (Utilities|Time|SetTimerbyEvent (EventDispatchers|CreateEvent :!event RegenGold) 1.0 true))
    (:then_1
      (Variables|Default|SetGold (Variables|Default|GetDefaultGold)))))

(event Collision|EventActorBeginOverlap
  (params (OtherActor :type Actor%20Object%20Reference)))

(event EventTick
  (params (DeltaSeconds :type Float%20%28single-precision%29)))

(event Input|KeyboardEvents|B
  (params (Key :type Key%20Structure :default "None"))
  (:Pressed
    (bind _thing (CallFunction|GetArray))
    (Utilities|Array|AddUnique _thing self)
    (Development|PrintString (Utilities|String|ToString(Integer) (Utilities|Array|Length (Variables|Default|GetARrray))))
    (for _array_element (Variables|Default|GetARrray)
      (Development|PrintString (Utilities|GetDisplayName _array_element)))))

(event Input|AxisEvents|InputAxisMoveForward
  (params (AxisValue :type Float%20%28single-precision%29))
  (Transformation|AddActorLocalOffset (* (* (* (Transformation|GetActorForwardVector) AxisValue) (/ (Utilities|Time|GetWorldDeltaSeconds) (Class|GameplayStatics|GetGlobalTimeDilation))) (Variables|Default|GetCameraPanSpeed)) false false))

(event Input|AxisEvents|InputAxisMoveRight
  (params (AxisValue :type Float%20%28single-precision%29))
  (Transformation|AddActorLocalOffset (* (* (* (Transformation|GetActorRightVector) AxisValue) (/ (Utilities|Time|GetWorldDeltaSeconds) (Class|GameplayStatics|GetGlobalTimeDilation))) (Variables|Default|GetCameraPanSpeed)) false false))

(event Input|KeyboardEvents|Z
  (params (Key :type Key%20Structure :default "None"))
  (:Pressed
    (Game|SpawnActorfromClass "/Game/Blueprints/BP_Archer_Projectile.BP_Archer_Projectile_C" (Transformation|GetWorldTransform (Variables|Default|GetCamera)) "Undefined" 0 0)))

(event Input|KeyboardEvents|J
  (params (Key :type Key%20Structure :default "None"))
  (:Pressed
    (Utilities|Time|SetGlobalTimeDilation 1.0)))

(event Input|KeyboardEvents|H
  (params (Key :type Key%20Structure :default "None"))
  (:Pressed
    (Utilities|Time|SetGlobalTimeDilation 0.3)))

(event Input|KeyboardEvents|G
  (params (Key :type Key%20Structure :default "None"))
  (:Pressed
    (Utilities|Time|SetGlobalTimeDilation 0.05)))

(event Input|KeyboardEvents|B
  (params (Key :type Key%20Structure :default "None"))
  (:Pressed
    (Class|TDGameMode|BuildNavMeshes (Variables|Default|GetGameMode))))

(event Input|KeyboardEvents|O
  (params (Key :type Key%20Structure :default "None"))
  (:Pressed
    (bind _outactors (Actor|GetAllActorsOfClass "/Game/Blueprints/BP_Tower.BP_Tower_C"))
    (for _array_element _outactors
      (CallFunction|ApplyGameplayEffectwithCallerMagnitude (Variables|/Script/TDTest.Tower|GetSystemComp _array_element) "/Game/GameplayAbilities/Attributes/GE_GrantExperience.GE_GrantExperience_C" "(TagName=\"attributes.experience.grant\")" 1e+02 true 0 _array_element))))

(fn ConstructionScript)

(fn RegenGold
  (Variables|Default|SetGold (+ (Variables|Default|GetGold) 1)))

(fn GetArray
  (return (Variables|Default|GetARrray)))