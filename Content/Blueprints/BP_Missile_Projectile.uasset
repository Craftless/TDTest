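; BP_Missile_Projectile is a missile projectile that deals area damage to enemies on impact.
; Its OnHit ignores the owner, then sphere-overlaps Pawns of class EnemyBase within Radius around the missile.
; Each overlapped enemy goes to DamageActor with the GE_GrantHealth effect class, despite that effect's healing-sounding name.
; It logs an error when nothing overlaps and destroys itself after any non-owner hit.
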(event Collision|EventActorBeginOverlap
  (params (OtherActor :type Actor%20Object%20Reference)))

(fn ConstructionScript)

(fn OnHit
  (params (HitActor :type Actor%20Object%20Reference))
  (if (not (== HitActor (Components|GetOwner)))
    (bind (_outactors _returnvalue) (Collision|SphereOverlapActors (Transformation|GetActorLocation) (Variables|Default|GetRadius) (Utilities|Array|MakeArray "ObjectTypeQuery3") "/Script/TDTest.EnemyBase" (Utilities|Array|MakeArray self)))
    (if _returnvalue
      (for _array_element _outactors
        (CallFunction|DamageActor _array_element "/Game/GameplayAbilities/Attributes/GE_GrantHealth.GE_GrantHealth_C"))
      (else
        (Utilities|PrintError "Could not find any actors to overlap")))
    (Actor|DestroyActor)))