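; A Blueprint function library of Gameplay Ability System helpers, plus a utility for attaching path components to actors.
; It builds effect specs with a tag-keyed SetByCaller magnitude and applies them to the source ASC or a target ASC.
; ExecuteModifier switches on modifier type to acquire or activate the modifier's ability on a target.
; AddPathToActor adds a component by class and passes it to the actor through an AddPathToUI interface message.
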(fn CreateGameplayEffectSpecwithCallerMagnitude
  (params (ASC :type Ability%20System%20Component%20Object%20Reference) (GameplayEffectClass :type Gameplay%20Effect%20Class%20Reference) (DataTag :type Gameplay%20Tag%20Structure) (Magnitude :type Float%20%28single-precision%29))
  (bind _returnvalue (Ability|GameplayEffect|AssignTagSetbyCallerMagnitude (GameplayEffects|MakeOutgoingSpec :self ASC :GameplayEffectClass GameplayEffectClass) DataTag Magnitude))
  (return _returnvalue))

(fn ApplyGameplayEffectwithCallerMagnitude
  (params (ASC :type Ability%20System%20Component%20Object%20Reference) (GEClass :type Gameplay%20Effect%20Class%20Reference) (DataTag :type Gameplay%20Tag%20Structure) (Magnitude :type Float%20%28single-precision%29) (TargetIsSelf :type Boolean) (Target%20ASC :type Ability%20System%20Component%20Object%20Reference) (__WorldContext1 :type Object%20Object%20Reference))
  (Utilities|IsValid ASC
    (:Is%20Valid
      (bind _gespec (CallFunction|CreateGameplayEffectSpecwithCallerMagnitude ASC GEClass DataTag Magnitude __WorldContext1))
      (if TargetIsSelf
        (GameplayEffects|ApplyGameplayEffectSpecToSelf ASC _gespec)
        (else
          (GameplayEffects|ApplyGameplayEffectSpecToTarget ASC _gespec Target%20ASC))))))

(fn ExecuteModifier
  (params (Modifier :type BP%20Modifier%20Object%20Reference) (Target :type Actor%20Object%20Reference) (AbilityLevel :type Integer))
  (bind _returnvalue (Ability|GetAbilitySystemComponent Target))
  (bind _gameplayability (Variables|/Game/GameplayAbilities/BP_Modifier.BP_Modifier_C|GetGameplayAbility Modifier))
  (switch Utilities|FlowControl|Switch|SwitchonEModifierType (Variables|/Game/GameplayAbilities/BP_Modifier.BP_Modifier_C|GetTypeOfModifier Modifier)
    (:NewEnumerator0
      (Class|GASFunctionLibrary|AcquireAbility _returnvalue _gameplayability AbilityLevel)
      (Abilities|TryActivateAbilitybyClass _returnvalue _gameplayability true))))

(fn AddPathtoActor
  (params (Actor :type Actor%20Object%20Reference) (PathClass :type BP%20Path%20Class%20Reference))
  (bind _returnvalue (Game|AddComponentbyClass Actor PathClass))
  (Class|IPathUser|AddPathtoUI(Message) Actor _returnvalue)
  (return _returnvalue))