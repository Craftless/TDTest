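; Actor that shows damage text in the world through a WBP_DamageText widget component.
; Text, font size and amount setters write to the widget when valid, otherwise buffer values that BeginPlay applies along with an OnAnimComplete binding.
; GetText and GetAmount read from the widget or fall back to the buffered values.
; AddAmount raises a live widget's amount by 1, ignoring InAmount, but adds InAmount when buffering.
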(event EventBeginPlay
  (bind _aswbp_damage_text (Utilities|Casting|CastToWBP_DamageText (UserInterface|GetUserWidgetObject (Variables|Default|GetWidget))))
  (Variables|Default|SetDamageText _aswbp_damage_text)
  (EventDispatchers|BindEventtoOnAnimComplete _aswbp_damage_text (EventDispatchers|CreateEvent :!event K2DestroyActor))
  (Default|SetText _aswbp_damage_text (Variables|Default|GetTextToDisplay))
  (Default|SetSize _aswbp_damage_text (Variables|Default|GetSize))
  (Default|SetAmount _aswbp_damage_text (Variables|Widget|GetWidgetAmount)))

(event Collision|EventActorBeginOverlap
  (params (OtherActor :type Actor%20Object%20Reference)))

(event EventTick
  (params (DeltaSeconds :type Float%20%28single-precision%29)))

(event EventSetText
  (params (InText :type Text%20%28by%20ref%29))
  (bind _damagetext (Variables|Default|GetDamageText)
    (:then
      (Default|SetText _damagetext InText))
    (:else
      (Variables|Default|SetTextToDisplay InText))))

(event EventSetFontSize
  (params (Size :type Integer))
  (bind _damagetext (Variables|Default|GetDamageText)
    (:then
      (Default|SetSize _damagetext Size))
    (:else
      (Variables|Default|SetSize Size))))

(event EventAddAmount
  (params (InAmount :type Integer))
  (bind _damagetext (Variables|Default|GetDamageText)
    (:then
      (Default|SetAmount _damagetext (+ (Variables|/Game/UI/WBP_DamageText.WBP_DamageText_C|GetAmount _damagetext) 1)))
    (:else
      (Variables|Widget|SetWidgetAmount (+ (Variables|Widget|GetWidgetAmount) InAmount)))))

(fn ConstructionScript)

(fn GetText
  (bind _damagetext (Variables|Default|GetDamageText))
  (return (select (Utilities|IsValid _damagetext) (Class|TextBlock|GetText (Variables|/Game/UI/WBP_DamageText.WBP_DamageText_C|GetDamageText _damagetext)) (Variables|Default|GetTextToDisplay))))

(fn GetAmount
  (bind _damagetext (Variables|Default|GetDamageText))
  (return (select (Utilities|IsValid _damagetext) (Variables|/Game/UI/WBP_DamageText.WBP_DamageText_C|GetAmount _damagetext) (Variables|Widget|GetWidgetAmount))))