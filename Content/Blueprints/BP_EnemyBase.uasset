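; Base tower-defense enemy Blueprint built on the Gameplay Ability System.
; On begin play it caches game mode and health bar, applies default speed and max health via set-by-caller effects, and creates a dynamic body material.
; Health loss flashes the body and shows damage text for the tower-owning player tracked as last damager.
; Death awards that player gold and notifies the game mode, while full experience applies a level-up effect.
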(event Custom|FlashBodyColour
  (params (Duration :type Float%20%28single-precision%29) (Value :type Linear%20Color%20Structure))
  (bind _dynmat (Variables|Default|GetDynMat)
    (:then
      (Rendering|Material|SetVectorParameterValue _dynmat (Variables|Colour|GetBodyColourParamName) Value :!class /Script/Engine.MaterialInstanceDynamic)
      (Utilities|FlowControl|Delay Duration)
      (Rendering|Material|SetVectorParameterValue (Variables|Default|GetDynMat) (Variables|Colour|GetBodyColourParamName) (Variables|Default|GetOriginalBodyColour) :!class /Script/Engine.MaterialInstanceDynamic))
    (:else)))

(event EventOnDeath
  (|CallParentFunction)
  (Utilities|FlowControl|Sequence
    (:then_0
      (bind _lastdamagedbyplayer (Variables|Default|GetLastDamagedByPlayer)
        (:then
          _)
        (:else
          (bind _astower (Utilities|Casting|CastToTower (Variables|Default|GetLastDamagedBy)))))
      (Class|PlayerPawn|AddGold _lastdamagedbyplayer (Variables|Default|GetGoldBounty)))
    (:then_1
      (Default|OnEnemyKilled (Variables|Default|GetGameMode) self)
      (Class|Pawn|DetachfromControllerPendingDestroy)
      (Actor|DestroyActor))))

(event EventTick
  (params (DeltaSeconds :type Float%20%28single-precision%29))
  (|CallParentFunction DeltaSeconds))

(event EventFinishedBeginPlay
  (Utilities|FlowControl|Sequence
    (:then_0
      (bind _asbp_tdclassic_game_mode (Utilities|Casting|CastToBP_TDClassicGameMode (Game|GetGameMode)))
      (Variables|Default|SetGameMode _asbp_tdclassic_game_mode))
    (:then_1
      (bind _aswbp_health_bar (Utilities|Casting|CastToWBP_HealthBar (UserInterface|GetUserWidgetObject (Variables|Default|GetWidget))))
      (Variables|Default|SetHealthBar _aswbp_health_bar))
    (:then_2
      (CallFunction|SetDefaultAttributeValues))
    (:then_3
      (bind _returnvalue (Rendering|Material|CreateDynamicMaterialInstance (Variables|Default|GetDynMatParent) "None" "None" :!class /Script/Engine.KismetMaterialLibrary))
      (bind _output_get (Variables|Default|SetDynMat _returnvalue))
      (Rendering|Material|SetMaterial (Variables|Character|GetMesh) 0 _output_get)
      (bind _returnvalue_2 (Rendering|Material|GetVectorParameterValue (Variables|Default|GetDynMat) (Variables|Colour|GetBodyColourParamName) :!class /Script/Engine.MaterialInstanceDynamic))
      (Variables|Default|SetOriginalBodyColour _returnvalue_2))))

(event EventOnMovementSpeedChanged
  (params (NewSpeed :type Float%20%28single-precision%29))
  (|CallParentFunction NewSpeed)
  (Variables|/Script/Engine.CharacterMovementComponent|SetMaxWalkSpeed (Variables|Character|GetCharacterMovement) NewSpeed))

(event EventOnHealthChanged
  (params (Health :type Float%20%28single-precision%29) (MaxHealth :type Float%20%28single-precision%29) (FullHealth :type Boolean) (PreviousHealth :type Float%20%28single-precision%29) (EffectInstigator :type Actor%20Object%20Reference))
  (|CallParentFunction Health MaxHealth FullHealth PreviousHealth EffectInstigator)
  (CallFunction|SetLastDamagedby EffectInstigator)
  (Default|SetPercentage (Variables|Default|GetHealthBar) (/ Health MaxHealth))
  (if (< Health PreviousHealth)
    (Utilities|FlowControl|Sequence
      (:then_0
        (CallFunction|FlashBodyColour 0.1 (Variables|Colour|GetDamagedColour)))
      (:then_1
        (bind _lastdamagedbyplayer (Variables|Default|GetLastDamagedByPlayer)
          (:then
            (bind _asbp_player_pawn (Utilities|Casting|CastToBP_PlayerPawn _lastdamagedbyplayer))
            (Class|DamageTextComponent|AddDamageIndicatorTextCLIENT (Variables|/Game/Blueprints/BP_PlayerPawn.BP_PlayerPawn_C|GetDamageText _asbp_player_pawn) "/Game/Blueprints/BP_DamageTextActor.BP_DamageTextActor_C" (Utilities|Text|ToText(Float) (- PreviousHealth Health) "HalfToEven" false true 1 324 0 0) (Transformation|GetWorldLocation (Variables|Default|GetWidget)) self))
          (:else))))))

(event EventOnExperienceChanged
  (params (Experience :type Float%20%28single-precision%29) (MaxExperience :type Float%20%28single-precision%29))
  (|CallParentFunction Experience MaxExperience)
  (if (>= Experience MaxExperience)
    (GameplayEffects|ApplyGameplayEffectToSelf :self (Variables|Default|GetSystemComp) :GameplayEffectClass "/Game/GameplayAbilities/Attributes/GE_LevelUp.GE_LevelUp_C" :Level (+ (.ReturnValue (Ability|Attribute|GetFloatAttributefromAbilitySystemComponent (Ability|GetAbilitySystemComponent 0) "(AttributeName=\"Level\",Attribute=/Script/TDTest.AttributeSetBase:Level,AttributeOwner=None)")) 1.0))))

(fn ConstructionScript)

(fn SetDefaultAttributeValues
  (Utilities|FlowControl|Sequence
    (:then_0
      (CallFunction|ApplyGameplayEffectwithCallerMagnitude "/Game/GameplayAbilities/Attributes/GE_SetMovementSpeed_Enemy.GE_SetMovementSpeed_Enemy_C" "(TagName=\"attributes.enemy.movementspeed.set\")" (Variables|Default|GetDefaultMovementSpeed)))
    (:then_1
      (CallFunction|ApplyGameplayEffectwithCallerMagnitude "/Game/GameplayAbilities/Attributes/GE_SetMaxHealth.GE_SetMaxHealth_C" "(TagName=\"attributes.maxhealth.set\")" (Variables|Default|GetDefaultMaxHealth)))))

(fn CreateGameplayEffectSpecwithCallerMagnitude
  (params (GameplayEffectClass :type Gameplay%20Effect%20Class%20Reference) (DataTag :type Gameplay%20Tag%20Structure) (Magnitude :type Float%20%28single-precision%29))
  (bind _returnvalue (Ability|GameplayEffect|AssignTagSetbyCallerMagnitude (GameplayEffects|MakeOutgoingSpec :self (Variables|Default|GetSystemComp) :GameplayEffectClass GameplayEffectClass) DataTag Magnitude))
  (return _returnvalue))

(fn ApplyGameplayEffectwithCallerMagnitude
  (params (GEClass :type Gameplay%20Effect%20Class%20Reference) (DataTag :type Gameplay%20Tag%20Structure) (Magnitude :type Float%20%28single-precision%29))
  (bind _gespec (CallFunction|CreateGameplayEffectSpecwithCallerMagnitude GEClass DataTag Magnitude))
  (GameplayEffects|ApplyGameplayEffectSpecToSelf (Variables|Default|GetSystemComp) _gespec))

(fn SetLastDamagedby
  (params (LastDamagedBy :type Actor%20Object%20Reference))
  (Utilities|IsValid LastDamagedBy
    (:Is%20Valid
      (bind _astower (Utilities|Casting|CastToTower LastDamagedBy)
        (:then
          (Variables|Default|SetLastDamagedByPlayer (Variables|/Script/TDTest.Tower|GetOwnerPlayer _astower)))
        (:CastFailed
          _))
      (Variables|Default|SetLastDamagedBy LastDamagedBy))))