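; Base AI controller for enemies that starts the enemy behavior tree and seeds its blackboard.
; On BeginPlay it loads BB_EnemyBase, runs BT_EnemyBase, then writes the BP_PathTile_End location as the end-point vector along with a hard-coded float key.
; On possess it caches the pawn as ControlledTower only if it casts to BP_Tower, despite the controller's enemy naming.
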(event EventBeginPlay
  (Utilities|FlowControl|Sequence
    (:then_0
      (bind _blackboardcomponent (Class|AIController|UseBlackboard "/Game/AI/BB_EnemyBase.BB_EnemyBase"))
      (Variables|Default|SetBBComp _blackboardcomponent)
      (AI|RunBehaviorTree "/Game/AI/BT_EnemyBase.BT_EnemyBase"))
    (:then_1
      (CallFunction|Initialise))))

(event EventTick
  (params (DeltaSeconds :type Float%20%28single-precision%29)))

(event EventPossess
  (params (PossessedPawn :type Pawn%20Object%20Reference))
  (bind _asbp_tower (Utilities|Casting|CastToBP_Tower PossessedPawn))
  (Variables|Default|SetControlledTower _asbp_tower))

(fn ConstructionScript)

(fn Initialise
  (Utilities|FlowControl|Sequence
    (:then_0
      (bind _bbcomp (Variables|Default|GetBBComp)
        (:then
          (bind _returnvalue (Actor|GetActorOfClass "/Game/Blueprints/BP_PathTIle_End.BP_PathTile_End_C"))
          (AI|Components|Blackboard|SetValueasVector _bbcomp (Variables|Default|GetEndPointKeyName) (Transformation|GetActorLocation _returnvalue)))
        (:else)))
    (:then_1
      (AI|Components|Blackboard|SetValueasFloat _bbcomp (Utilities|Name|MakeLiteralName "FloatKey") 69.0))))