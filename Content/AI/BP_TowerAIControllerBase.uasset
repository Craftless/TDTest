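; Base AI controller for towers that runs a behavior tree and chooses which sensed enemy to attack.
; Delegates from the possessed tower maintain the sensed-enemy list and supply attack time, which is cached until the Blackboard exists.
; Every tick it retargets by the tower's Normal, Closest or Weakest mode, writing the result to the Blackboard.
; Optional smart targeting first picks any enemy whose attribute ratio is low.
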(event EventBeginPlay
  (Utilities|FlowControl|Sequence
    (:then_0
      (bind _blackboardcomponent (Class|AIController|UseBlackboard "/Game/AI/BB_TowerBase.BB_TowerBase"))
      (Variables|Default|SetBBComp _blackboardcomponent)
      (AI|RunBehaviorTree "/Game/AI/BT_TowerBase.BT_TowerBase")
      (Development|PrintString "Started tower"))
    (:then_1
      (CallFunction|Initialise))))

(event EventPossess
  (params (PossessedPawn :type Pawn%20Object%20Reference))
  (bind _asbp_tower (Utilities|Casting|CastToBP_Tower PossessedPawn))
  (bind _output_get (Variables|Default|SetControlledTower _asbp_tower))
  (Utilities|FlowControl|Sequence
    (:then_0
      (EventDispatchers|BindEventtoOnNewAttackSpeedDelegate _output_get (EventDispatchers|CreateEvent :!event OnNewAttackSpeed)))
    (:then_1
      (EventDispatchers|BindEventtoOnStartedSensingEnemy _output_get (EventDispatchers|CreateEvent :!event OnStartedSensingEnemy)))
    (:then_2
      (EventDispatchers|BindEventtoOnStoppedSensingEnemy _output_get (EventDispatchers|CreateEvent :!event OnStoppedSensingEnemy)))))

(event EventTick
  (params (DeltaSeconds :type Float%20%28single-precision%29))
  (|CallParentFunction DeltaSeconds)
  (CallFunction|UpdateEnemy))

(fn ConstructionScript)

(fn OnNewAttackSpeed
  (params (NewAttackSpeed :type Float%20%28single-precision%29) (NewAttackTime :type Float%20%28single-precision%29))
  (bind _bbcomp (Variables|Default|GetBBComp)
    (:then
      (AI|Components|Blackboard|SetValueasFloat _bbcomp (Variables|Default|GetAttackTimeKeyName) NewAttackTime))
    (:else
      (Variables|Default|SetTempAtkTime NewAttackTime))))

(fn Initialise
  (bind _tempatktime (Variables|Default|GetTempAtkTime))
  (Utilities|FlowControl|Sequence
    (:then_0
      (bind _bbcomp (Variables|Default|GetBBComp)
        (:then
          (Utilities|FlowControl|Sequence
            (:then_0
              (if (!= _tempatktime -1.0)
                (AI|Components|Blackboard|SetValueasFloat _bbcomp (Variables|Default|GetAttackTimeKeyName) _tempatktime)))
            (:then_1
              (AI|Components|Blackboard|SetValueasBool _bbcomp (Variables|Default|GetCanAttackKeyName) true))))
        (:else)))))

(fn OnStartedSensingEnemy
  (params (Enemy :type Enemy%20Base%20Object%20Reference))
  (bind _sensedenemies (Variables|Default|GetSensedEnemies))
  (Utilities|Array|AddUnique _sensedenemies Enemy)
  (bind _enemy (CallFunction|GetEnemy _sensedenemies))
  (bind _output_get (Variables|Default|SetEnemy _enemy))
  (AI|Components|Blackboard|SetValueasObject (Variables|Default|GetBBComp) (Variables|Default|GetEnemyKeyName) _output_get)
  (return))

(fn OnStoppedSensingEnemy
  (params (Enemy :type Enemy%20Base%20Object%20Reference))
  (bind _returnvalue (Utilities|Array|RemoveItem (Variables|Default|GetSensedEnemies) Enemy))
  (if _returnvalue
    (CallFunction|UpdateEnemy)
    (else
      (Development|PrintString "Error: Attempting to remove a non-existent item" true true "(R=1.000000,G=0.000000,B=0.000000,A=1.000000)"))))

(fn GetEnemy
  (params (Array :type Array%20of%20Enemy%20Base%20Object%20References))
  (if (Variables|Default|GetSmartTargeting)
    (for _array_element Array
      (if (Math|Boolean|ANDBoolean (.bSuccessfullyFoundAttribute (Ability|Attribute|GetFloatAttribute _array_element "(AttributeName=\"Health\",Attribute=/Script/TDTest.AttributeSetBase:Health,AttributeOwner=None)")) (.bSuccessfullyFoundAttribute (Ability|Attribute|GetFloatAttribute _array_element "(AttributeName=\"MaxHealth\",Attribute=/Script/TDTest.AttributeSetBase:MaxHealth,AttributeOwner=None)")) (<= (/ (.ReturnValue (Ability|Attribute|GetFloatAttribute _array_element "(AttributeName=\"Health\",Attribute=/Script/TDTest.AttributeSetBase:Health,AttributeOwner=None)")) (.ReturnValue (Ability|Attribute|GetFloatAttribute _array_element "(AttributeName=\"MaxHealth\",Attribute=/Script/TDTest.AttributeSetBase:MaxHealth,AttributeOwner=None)"))) 0.2))
        (return _array_element))))
  (switch Utilities|FlowControl|Switch|SwitchonETargetingMode (Variables|/Script/TDTest.Tower|GetTargetingMode (Variables|Default|GetControlledTower))
    (:Normal
      (return (Utilities|Array|Get(acopy) Array)))
    (:Closest
      (for _array_element_2 Array
        (Utilities|IsValid (.enemybase (LocalVariables|GetClosestEnemy))
          (:Is%20Valid
            (if (< (Class|KismetMathLibrary|VectorDistanceSquared (Transformation|GetActorLocation _array_element_2) (Transformation|GetActorLocation (Variables|Default|GetControlledTower))) (.distancesquared (LocalVariables|GetClosestEnemy)))
              (LocalVariables|SetClosestEnemy (Utilities|Struct|MakeFEnemyDist _array_element_2 (Class|KismetMathLibrary|VectorDistanceSquared (Transformation|GetActorLocation _array_element_2) (Transformation|GetActorLocation (Variables|Default|GetControlledTower)))) :!label _label)))
          (:Is%20Not%20Valid
            (goto _label))))
      (return (.enemybase (LocalVariables|GetClosestEnemy))))
    (:Weakest
      (for _array_element_3 Array
        (Utilities|IsValid (.enemybase (LocalVariables|GetWeakestEnemy))
          (:Is%20Valid
            (if (< (.ReturnValue (Ability|Attribute|GetFloatAttribute _array_element_3 "(AttributeName=\"Health\",Attribute=/Script/TDTest.AttributeSetBase:Health,AttributeOwner=None)")) (.distancesquared (LocalVariables|GetWeakestEnemy)))
              (LocalVariables|SetWeakestEnemy (Utilities|Struct|MakeFEnemyDist _array_element_3 (.ReturnValue (Ability|Attribute|GetFloatAttribute _array_element_3 "(AttributeName=\"Health\",Attribute=/Script/TDTest.AttributeSetBase:Health,AttributeOwner=None)"))) :!label _label_2)))
          (:Is%20Not%20Valid
            (goto _label_2))))
      (return (.enemybase (LocalVariables|GetWeakestEnemy))))))

(fn UpdateEnemy
  (bind _bbcomp (Variables|Default|GetBBComp))
  (bind _enemykeyname (Variables|Default|GetEnemyKeyName))
  (if (> (Utilities|Array|Length (Variables|Default|GetSensedEnemies)) 0)
    (bind _enemy (CallFunction|GetEnemy (Variables|Default|GetSensedEnemies)))
    (bind _output_get (Variables|Default|SetEnemy _enemy))
    (AI|Components|Blackboard|SetValueasObject _bbcomp _enemykeyname _output_get)
    (else
      (AI|Components|Blackboard|ClearValue _bbcomp _enemykeyname)
      (Variables|Default|SetEnemy 0))))

(fn ChangeCanAttack
  (params (BoolValue :type Boolean))
  (bind _blackboard (Variables|Default|GetBlackboard)
    (:then
      (AI|Components|Blackboard|SetValueasBool _blackboard (Variables|Default|GetCanAttackKeyName) BoolValue))
    (:else)))