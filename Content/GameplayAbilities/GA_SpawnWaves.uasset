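; Gameplay ability for spawning tower-defense enemy waves, currently unfinished.
; On activation it splits the first WaveLayout entry from BP_TDClassicGameMode into characters, then empties them in a while loop that starts delays without waiting on them.
; Disconnected logic reads 'B' as a basic enemy and numbers as pauses, with retries for blocked spawns, and holds the EndAbility call.
; SpawnEnemy spawns at StartTile minus the class's offset, failing on collision.
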(event Ability|EventActivateAbility
  (bind _asbp_tdclassic_game_mode (Utilities|Casting|CastToBP_TDClassicGameMode (Game|GetGameMode)))
  (Variables|Default|SetGameMode _asbp_tdclassic_game_mode)
  (bind _output_get (Variables|Default|SetArrayed (Utilities|String|GetCharacterArrayfromString (Utilities|String|ToString(Text) (Utilities|Array|Get(acopy) (Variables|/Game/Blueprints/BP_TDClassicGameMode.BP_TDClassicGameMode_C|GetWaveLayout _asbp_tdclassic_game_mode))))))
  (while (> (Utilities|Array|Length _output_get) 0)
    (Utilities|FlowControl|Sequence
      (:then_0
        (Ability|Tasks|WaitDelay 5.0))
      (:then_1
        (Utilities|Array|RemoveIndex (Variables|Default|GetArrayed))
        (Development|PrintString "saEIONFOIK")))))

(event Ability|EventOnEndAbility
  (params (bWasCancelled :type Boolean)))

(fn SpawnEnemy
  (params (EnemyClass :type Enemy%20Base%20Class%20Reference))
  (bind _gamemode (Variables|Default|GetGameMode))
  (bind _starttile (Variables|/Game/Blueprints/BP_TDClassicGameMode.BP_TDClassicGameMode_C|GetStartTile _gamemode))
  (bind _returnvalue (Transformation|GetActorTransform _starttile))
  (bind _returnvalue_2 (Game|SpawnActorfromClass EnemyClass (Math|Transform|MakeTransform (- (.location _returnvalue) (.SpawningOffset (Utilities|GetClassDefaults EnemyClass))) (.rotation _returnvalue) (.scale _returnvalue)) "DontSpawnIfColliding" 0 0))
  (return (Utilities|IsValid _returnvalue_2)))