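; Burn modifier gameplay ability that adds a damage-over-duration burn effect to its target's spawned projectile.
; On activation it reads Damage and Duration from CT_Modifier_Burn at the ability level.
; It builds a GE_Burn spec with negated damage and duration as SetByCaller magnitudes, then adds it uniquely to the projectile's DamageActorConditionalModifiers.
; The graph does nothing without a valid projectile and never calls EndAbility.
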(event Ability|EventActivateAbility
  (bind _tower_projectile_shooter (CallFunction|GetTarget))
  (bind _spawnedprojectile (Variables|/Game/Blueprints/BP_Tower_ProjectileShooter.BP_Tower_ProjectileShooter_C|GetSpawnedProjectile _tower_projectile_shooter)
    (:then
      (bind _outxy (DataTable|EvaluateCurveTableRow "/Game/GameplayAbilities/Modifiers/CT_Modifier_Burn.CT_Modifier_Burn" "Damage" (Math|Conversions|ToFloat(Integer) (Ability|GetAbilityLevel)))
        (:RowFound
          (bind _gespec (Default|CreateGameplayEffectSpecwithCallerMagnitude _tower_projectile_shooter "/Game/GameplayAbilities/Modifiers/GE_Burn.GE_Burn_C" "(TagName=\"modifiers.burn.damage\")" (* _outxy -1.0)))
          (bind _outxy_2 (DataTable|EvaluateCurveTableRow "/Game/GameplayAbilities/Modifiers/CT_Modifier_Burn.CT_Modifier_Burn" "Duration" (Math|Conversions|ToFloat(Integer) (Ability|GetAbilityLevel)))
            (:RowFound
              (bind _returnvalue (Ability|GameplayEffect|AssignTagSetbyCallerMagnitude _gespec "(TagName=\"modifiers.burn.duration\")" _outxy_2))
              (Utilities|Array|AddUnique (Variables|/Game/Blueprints/BP_Tower_GenericProjectile.BP_Tower_GenericProjectile_C|GetDamageActorConditionalModifiers _spawnedprojectile) _returnvalue))))))
    (:else)))

(event Ability|EventOnEndAbility
  (params (bWasCancelled :type Boolean)))